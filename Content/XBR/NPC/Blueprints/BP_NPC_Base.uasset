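; BP_NPC_Base is a base NPC Blueprint that shows a head info widget above the character.
; On BeginPlay it looks up its row in Table_NPCInformation by NPCName and feeds name, HP and MP values with visibility flags to the widget, starting both bars at max.
; Each Tick, FFacePlayer yaws the widget toward the player camera.
; Clicking the skeletal mesh only prints a placeholder "Hello".
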(event `self.SkeletalMesh.OnClicked`
  (params (TouchedComponent :type "PrimitiveComponent Object Reference") (ButtonPressed :type "Key Structure"))
  (`KismetSystemLibrary.PrintString` "Hello"))

(event `self.ReceiveBeginPlay`
  (bind _asui_npchead_inf (cast `/Game/XBR/UI/UI_NPCHeadInf` (`WidgetComponent.GetUserWidgetObject` (`self.Widget`))))
  (set `self.NPCHeadInf` _asui_npchead_inf)
  (bind _returnvalue (`|GetDataTableRow` "/Game/XBR/NPC/Blueprints/Struct/Table_NPCInformation.Table_NPCInformation" (`self.NPCName`))
    (:`then`
      (bind _npcheadinf (`self.NPCHeadInf`)
        (:`then`
          (bind (_id _name _maxhp _maxmp _isshownpcname _isshowhp _isshowmp) (break `/Game/XBR/NPC/Blueprints/Struct/S_NPCInformation` _returnvalue))
          (`/Game/XBR/UI/UI_NPCHeadInf.F Show Head Inf` _npcheadinf _name _isshownpcname _maxhp _maxhp _isshowhp _maxmp _maxmp _isshowmp))
        (:`else`)))))

(event `self.ReceiveTick`
  (params (DeltaSeconds :type "Float (single-precision)"))
  (`self.F_FacePlayer`))

(fn `F_FacePlayer`
  (bind _widget (`self.Widget`))
  (`SceneComponent.K2_SetWorldRotation` _widget (`KismetMathLibrary.MakeRotator` 0.0 0.0 (.yaw (`KismetMathLibrary.FindLookAtRotation` (`SceneComponent.K2_GetComponentLocation` _widget) (`self.K2_GetActorLocation` (`GameplayStatics.GetPlayerCameraManager` 0))))) false false))

(fn `UserConstructionScript`)